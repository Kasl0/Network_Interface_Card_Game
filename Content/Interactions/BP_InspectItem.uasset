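; BP_InspectItem is an interaction Blueprint, named for inspectable items, that responds when an interaction starts.
; Its StartInteraction override runs the parent logic, casts the player 0 pawn to BP_GameCharacter and calls OnInteract with that character.
; The Inspect event is an empty stub, and the construction script only calls its parent.
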(event EventBeginPlay
  (|CallParentFunction) ; This node is disabled and will not be called.\nDrag off pins to build functionality.
)

(event Collision|EventActorBeginOverlap
  (params (OtherActor :type Actor%20Object%20Reference))
  (|CallParentFunction OtherActor) ; This node is disabled and will not be called.\nDrag off pins to build functionality.
)

(event EventTick
  (params (DeltaSeconds :type Float%20%28single-precision%29))
  (|CallParentFunction DeltaSeconds) ; This node is disabled and will not be called.\nDrag off pins to build functionality.
)

(event EventInspect
  (params (Character :type BP%20Game%20Character%20Object%20Reference) (Inspected%20Item :type Static%20Mesh%20Object%20Reference) (Item%20Name :type Text) (Item%20Description :type Text)))

(fn ConstructionScript
  (|CallParentFunction))

(fn StartInteraction
  (|CallParentFunction)
  (bind _asbp_game_character (Utilities|Casting|CastToBP_GameCharacter (Game|Player|GetPlayerPawn 0)))
  (CallFunction|OnInteract _asbp_game_character))