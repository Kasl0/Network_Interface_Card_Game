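; BP_CardActor is a card actor that displays a minion's name, description, attack, health and image from its MinionData.
; On BeginPlay it fills the text components and creates a dynamic material for the image, setting its Image texture parameter with no texture wired in.
; SetAttackText and SetHealthText color values green above base and red below, leaving the color untouched when equal.
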(event EventBeginPlay
  (Rendering|Components|TextRender|SetText (Variables|Default|GetName) (Variables|/Script/NICGame.CardData|GetCardName (Variables|Default|GetMinionData)))
  (Rendering|Components|TextRender|SetText (Variables|Default|GetDescription) (Variables|/Script/NICGame.CardData|GetCardDescription (Variables|Default|GetMinionData)))
  (CallFunction|SetAttackText)
  (CallFunction|SetHealthText)
  (bind _returnvalue (Rendering|Material|CreateDynamicMaterialInstance (Variables|Default|GetImage) 0 "/Game/CardActor/CardImageMaterial.CardImageMaterial" "None" :!class /Script/Engine.PrimitiveComponent))
  (Rendering|Material|SetTextureParameterValue _returnvalue "Image" 0))

(event Collision|EventActorBeginOverlap
  (params (OtherActor :type Actor%20Object%20Reference)))

(event EventTick
  (params (DeltaSeconds :type Float%20%28single-precision%29)))

(fn ConstructionScript)

(fn SetAttackText
  (bind _miniondata (Variables|Default|GetMinionData))
  (bind _baseattack (Variables|/Script/NICGame.Minion|GetBaseAttack _miniondata))
  (bind _returnvalue (Class|Minion|GetAttack _miniondata))
  (Rendering|Components|TextRender|SetText (Variables|Default|GetAttack) (Utilities|Text|ToText(Integer) _returnvalue))
  (if (> _returnvalue _baseattack)
    (Rendering|Components|TextRender|SetTextRenderColor (Variables|Default|GetAttack) (Math|Color|MakeColor 0 1 0 1))
    (elif (< _returnvalue _baseattack)
      (Rendering|Components|TextRender|SetTextRenderColor (Variables|Default|GetAttack) (Math|Color|MakeColor 0 0 1 1)))))

(fn SetHealthText
  (bind _miniondata (Variables|Default|GetMinionData))
  (bind _basehealth (Variables|/Script/NICGame.Minion|GetBaseHealth _miniondata))
  (bind _returnvalue (Class|Minion|GetCurrentHealth _miniondata))
  (Rendering|Components|TextRender|SetText (Variables|Default|GetHealth) (Utilities|Text|ToText(Integer) _returnvalue))
  (if (> _returnvalue _basehealth)
    (Rendering|Components|TextRender|SetTextRenderColor (Variables|Default|GetHealth) (Math|Color|MakeColor 0 1 0 1))
    (elif (< _returnvalue _basehealth)
      (Rendering|Components|TextRender|SetTextRenderColor (Variables|Default|GetHealth) (Math|Color|MakeColor 0 0 1 1)))))