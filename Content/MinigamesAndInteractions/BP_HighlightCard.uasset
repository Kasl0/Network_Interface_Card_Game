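; BP_HighlightCard is an interactable actor that highlights its mesh and responds to clicks while another actor overlaps it.
; Overlap and cursor events set two flags; when both are true, the mesh gets an overlay material and the cursor becomes a hand, otherwise both reset.
; A click in that state calls StartInteraction, and ending overlap calls EndInteraction.
; Both interaction functions are empty here.
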(event EventBeginPlay)

(event EventTick
  (params (DeltaSeconds :type Float%20%28single-precision%29)))

(event MouseInput|EventActorEndCursorOver
  (bind _returnvalue (Game|GetPlayerController 0))
  (bind _staticmesh (Variables|Default|GetStaticMesh))
  (Variables|Default|SetCursorOver false)
  (if (and (Variables|Default|GetOverlap) (Variables|Default|GetCursorOver))
    (Rendering|Material|SetOverlayMaterial _staticmesh (Variables|Default|GetHighlightMaterial) :!class /Script/Engine.MeshComponent)
    (Variables|/Script/Engine.PlayerController|SetCurrentMouseCursor _returnvalue "Hand")
    (else
      (Rendering|Material|SetOverlayMaterial _staticmesh 0 :!class /Script/Engine.MeshComponent)
      (Variables|/Script/Engine.PlayerController|SetCurrentMouseCursor _returnvalue "Default"))))

(event MouseInput|EventActorBeginCursorOver
  (bind _returnvalue (Game|GetPlayerController 0))
  (bind _staticmesh (Variables|Default|GetStaticMesh))
  (Variables|Default|SetCursorOver true)
  (if (and (Variables|Default|GetOverlap) (Variables|Default|GetCursorOver))
    (Rendering|Material|SetOverlayMaterial _staticmesh (Variables|Default|GetHighlightMaterial) :!class /Script/Engine.MeshComponent)
    (Variables|/Script/Engine.PlayerController|SetCurrentMouseCursor _returnvalue "Hand")
    (else
      (Rendering|Material|SetOverlayMaterial _staticmesh 0 :!class /Script/Engine.MeshComponent)
      (Variables|/Script/Engine.PlayerController|SetCurrentMouseCursor _returnvalue "Default"))))

(event Collision|EventActorBeginOverlap
  (params (OtherActor :type Actor%20Object%20Reference))
  (bind _returnvalue (Game|GetPlayerController 0))
  (bind _staticmesh (Variables|Default|GetStaticMesh))
  (Variables|Default|SetOverlap true)
  (if (and (Variables|Default|GetOverlap) (Variables|Default|GetCursorOver))
    (Rendering|Material|SetOverlayMaterial _staticmesh (Variables|Default|GetHighlightMaterial) :!class /Script/Engine.MeshComponent)
    (Variables|/Script/Engine.PlayerController|SetCurrentMouseCursor _returnvalue "Hand")
    (else
      (Rendering|Material|SetOverlayMaterial _staticmesh 0 :!class /Script/Engine.MeshComponent)
      (Variables|/Script/Engine.PlayerController|SetCurrentMouseCursor _returnvalue "Default"))))

(event Collision|EventActorEndOverlap
  (params (OtherActor :type Actor%20Object%20Reference))
  (bind _returnvalue (Game|GetPlayerController 0))
  (bind _staticmesh (Variables|Default|GetStaticMesh))
  (CallFunction|EndInteraction)
  (Variables|Default|SetOverlap false)
  (if (and (Variables|Default|GetOverlap) (Variables|Default|GetCursorOver))
    (Rendering|Material|SetOverlayMaterial _staticmesh (Variables|Default|GetHighlightMaterial) :!class /Script/Engine.MeshComponent)
    (Variables|/Script/Engine.PlayerController|SetCurrentMouseCursor _returnvalue "Hand")
    (else
      (Rendering|Material|SetOverlayMaterial _staticmesh 0 :!class /Script/Engine.MeshComponent)
      (Variables|/Script/Engine.PlayerController|SetCurrentMouseCursor _returnvalue "Default"))))

(event MouseInput|EventActorOnClicked
  (params (ButtonPressed :type Key%20Structure :default "None"))
  (if (and (Variables|Default|GetOverlap) (Variables|Default|GetCursorOver))
    (CallFunction|StartInteraction)))

(fn ConstructionScript)

(fn StartInteraction)

(fn EndInteraction)