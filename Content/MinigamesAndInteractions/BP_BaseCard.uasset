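; BP_BaseCard is an interactable card actor that opens an inspection view when a character interacts with it.
; On interact it spawns a BP_InspectedCard at a location far from the world origin, likely to isolate it from the level.
; It copies its inspection rotation, scale and zoom limits onto that actor, then passes the character, item name and description through InspectMessage.
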(event EventBeginPlay)

(event Collision|EventActorBeginOverlap
  (params (OtherActor :type Actor%20Object%20Reference)))

(event EventTick
  (params (DeltaSeconds :type Float%20%28single-precision%29)))

(event EventOnInteract
  (params (Character :type BP%20Game%20Character%20Object%20Reference))
  (bind _returnvalue (Game|SpawnActorfromClass "/Game/MinigamesAndInteractions/Inspect/BP_InspectedCard.BP_InspectedCard_C" (Math|Transform|MakeTransform "100000000.000000,0.000000,0.000000") "Undefined" "MultiplyWithRoot" 0 0))
  (Default|SetInspectRotation _returnvalue (Variables|Public|Interaction|Inspection|GetItem%20Inspection%20Rotation))
  (Default|SetInspectScale _returnvalue (Variables|Public|Interaction|Inspection|GetItem%20Inspection%20Scale))
  (Default|SetInspectMinZoom _returnvalue (Variables|Public|Interaction|Inspection|GetItem%20Inspection%20Min%20Zoom))
  (Default|SetInspectMaxZoom _returnvalue (Variables|Public|Interaction|Inspection|GetItem%20Inspection%20Max%20Zoom))
  (Class|InteractInterface|Inspect(Message) _returnvalue Character 0 (Variables|Public|Mesh|GetItem%20Name) (Variables|Public|Mesh|GetItem%20Description)))

(fn ConstructionScript)