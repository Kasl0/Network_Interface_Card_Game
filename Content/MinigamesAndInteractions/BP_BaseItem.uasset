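; BP_BaseItem is a base item actor that can open an inspection of itself when a character interacts with it.
; Its construction script applies the configured mesh and world scale to the StaticMesh component.
; If Inspect is set, OnInteract spawns a BP_InspectedItem far from the world origin.
; It passes that actor the inspection rotation and scale, then sends the character, mesh, name and description through InspectMessage.
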(event EventBeginPlay)

(event Collision|EventActorBeginOverlap
  (params (OtherActor :type Actor%20Object%20Reference)))

(event EventTick
  (params (DeltaSeconds :type Float%20%28single-precision%29)))

(event EventOnInteract
  (params (Character :type BP%20Game%20Character%20Object%20Reference))
  (if (Variables|Public|Interaction|Inspection|GetInspect?)
    (bind _returnvalue (Game|SpawnActorfromClass "/Game/MinigamesAndInteractions/Inspect/BP_InspectedItem.BP_InspectedItem_C" (Math|Transform|MakeTransform "100000000.000000,0.000000,0.000000") "Undefined" "MultiplyWithRoot" 0 0))
    (Default|SetInspectRotation _returnvalue (Variables|Public|Interaction|Inspection|GetItem%20Inspection%20Rotation))
    (Default|SetInspectScale _returnvalue (Variables|Public|Interaction|Inspection|GetItem%20Inspection%20Scale))
    (Class|InteractInterface|Inspect(Message) _returnvalue Character (Variables|/Script/Engine.StaticMeshComponent|GetStaticMesh (Variables|Default|GetStaticMesh)) (Variables|Public|Mesh|GetItem%20Name) (Variables|Public|Mesh|GetItem%20Description))))

(fn ConstructionScript
  (bind _staticmesh (Variables|Default|GetStaticMesh))
  (Components|StaticMesh|SetStaticMesh (Variables|Default|GetStaticMesh) (Variables|Public|Mesh|GetItem%20Mesh))
  (Transformation|SetWorldTransform _staticmesh (Math|Transform|MakeTransform (Transformation|GetWorldLocation _staticmesh) (Transformation|GetWorldRotation _staticmesh) (Variables|Public|Mesh|GetItem%20Scale)) false false))